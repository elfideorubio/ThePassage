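; BP_IslandYthen is an island actor that triggers the move to the credits level once the final stage is reached and the boat is at the island.
; FinalStage activates three particle systems and sets the first flag, while a sphere overlap with BP_Boat sets and clears the second.
; A looping one-second timer started on BeginPlay checks both flags and opens the "Shayan" level when both are true.
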(event `self.ReceiveBeginPlay`
  (`KismetSystemLibrary.K2_SetTimerDelegate` (delegate `OpenCredits`) 1.0 true))

(event `OpenCredits`
  (if (and (`self.CanMoveToCredits1`) (`self.CanMoveToCredits2`))
    (`GameplayStatics.OpenLevel` "Shayan")))

(event `FinalStage`
  (`ActorComponent.Activate` (`self.ParticleSystemComponent0`) false)
  (`ActorComponent.Activate` (`self.ParticleSystemComponent1`) false)
  (`ActorComponent.Activate` (`self.ParticleSystemComponent2`) false)
  (set `self.CanMoveToCredits1` true))

(event `self.Sphere.OnComponentBeginOverlap`
  (params (OverlappedComponent :type "PrimitiveComponent Object Reference") (OtherActor :type "Actor Object Reference") (OtherComp :type "PrimitiveComponent Object Reference") (OtherBodyIndex :type Integer) (bFromSweep :type Boolean) (SweepResult :type "HitResult Structure (by ref)"))
  (cast `/Game/Core/Characters/Boat/BP_Boat` OtherActor)
  (bind _output_get (set `self.CanMoveToCredits2` true))
  (`KismetSystemLibrary.PrintString` (`KismetStringLibrary.Conv_BoolToString` _output_get)))

(event `self.Sphere.OnComponentEndOverlap`
  (params (OverlappedComponent :type "PrimitiveComponent Object Reference") (OtherActor :type "Actor Object Reference") (OtherComp :type "PrimitiveComponent Object Reference") (OtherBodyIndex :type Integer))
  (cast `/Game/Core/Characters/Boat/BP_Boat` OtherActor)
  (bind _output_get (set `self.CanMoveToCredits2` false))
  (`KismetSystemLibrary.PrintString` (`KismetStringLibrary.Conv_BoolToString` _output_get)))

(fn `UserConstructionScript`)