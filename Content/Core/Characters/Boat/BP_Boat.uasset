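; BP_Boat is a drivable boat with its own kinematic movement, steered by input axes, plus a camera gimbal that only yaws.
; Each tick it yaws by steering, sums throttle thrust and velocity-squared drag into acceleration, adds that to velocity without delta-time scaling, and offsets the actor without sweep.
; A collision overlap zeroes velocity, applies a fixed world -X force to the mesh and prints a debug message.
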(event `self.ReceiveBeginPlay`)

(event `InputAxis|LookUp`
  (params (AxisValue :type "Float (single-precision)"))
  ;[1 1 1] Boat Camera Input Binding
)

(event `InputAxis|Turn`
  (params (AxisValue :type "Float (single-precision)"))
  ;[1 1 1] Boat Camera Input Binding
  (`SceneComponent.K2_AddLocalRotation` (`self.CameraGimbal`) (`KismetMathLibrary.MakeRotator` 0.0 0.0 (* AxisValue (`GameplayStatics.GetWorldDeltaSeconds`) 20.0)) false false))

(event `InputAxis|MoveForward`
  (params (AxisValue :type "Float (single-precision)"))
  (if (>= AxisValue 0.0)
    (set `self.ForwardThrottle` AxisValue)
    (else
      (set `self.ForwardThrottle` -0.1))))

(event `InputAxis|MoveRight`
  (params (AxisValue :type "Float (single-precision)"))
  (set `self.SteeringThrottle` AxisValue))

(event `self.ReceiveTick`
  (params (DeltaSeconds :type "Float (single-precision)"))
  (`|ExecutionSequence`
    (:`then_0`
      (bind _output_get (set `self.RotationAngle` (* (`self.MaxDegreePerSecond`) (`self.SteeringThrottle`) DeltaSeconds)))
      (`self.K2_AddActorWorldRotation` (`KismetMathLibrary.MakeRotator` 0.0 0.0 _output_get)))
    (:`then_1`
      ;[1 1 1] Setting Force
      (bind _output_get_2 (set `self.Force` (* (* (`SceneComponent.GetForwardVector` (`self.ForceLocation`)) (`self.BoatMaxDrivingForce`)) (`self.ForwardThrottle`))))
      (bind _newparam (`self.GetResistance`))
      (set `self.Force` (+ _output_get_2 _newparam))
      ;[1 1 1] Set Acceleration according to Force
      (bind _output_get_3 (set `self.Acceleration` (/ _output_get_2 (`PrimitiveComponent.GetMass` (`self.BoatMesh`)))))
      ;[1 1 1] Setting Velocity
      (bind _output_get_4 (set `self.Velocity` (+ _output_get_3 (`self.Velocity`))))
      ;[1 1 1] Add Force to Boat
      (bind _output_get_5 (set `self.Translation` (* _output_get_4 DeltaSeconds)))
      (`self.K2_AddActorWorldOffset` _output_get_5))))

(event `self.CollideDetector.OnComponentBeginOverlap`
  (params (OverlappedComponent :type "PrimitiveComponent Object Reference") (OtherActor :type "Actor Object Reference") (OtherComp :type "PrimitiveComponent Object Reference") (OtherBodyIndex :type Integer) (bFromSweep :type Boolean) (SweepResult :type "HitResult Structure (by ref)"))
  ;[1 1 1] set velocity to zero when hit something
  (set `self.Velocity` (`KismetMathLibrary.Vector_Zero`))
  (`PrimitiveComponent.AddForce` (`self.BoatMesh`) (-3000000.0 0.0 0.0) "None" false)
  (`KismetSystemLibrary.PrintString` "Force added"))

(fn `GetResistance`
  (returns (NewParam :type "Vector Structure"))
  (bind _velocity (`self.Velocity`))
  (return (* (* (`KismetMathLibrary.Normal` _velocity) (* (`KismetMathLibrary.VSizeSquared` _velocity) (`self.DragCoefficient`))) -1.0)))

(fn `UserConstructionScript`)