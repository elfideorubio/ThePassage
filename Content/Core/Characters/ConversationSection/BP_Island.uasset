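; BP_Island is an island actor that rises when play begins and detects the boat.
; A timeline, also triggerable through MoveIsland, lerps each update from the current location toward 130 units above it, so the offset compounds rather than following fixed endpoints.
; When the timeline finishes it sets HasFinishPlaying, which gates the sphere's begin and end overlap responses to BP_Boat, currently just debug prints.
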(event `self.ReceiveBeginPlay`
  (bind (_returnvalue_x _returnvalue_y _returnvalue_z) (`KismetMathLibrary.BreakVector` (`self.K2_GetActorLocation`)))
  (bind (_direction _islandspeed) (`Timeline|Timeline_0` :!label _label)
    (:`Update`
      (`self.K2_SetActorLocation` (`KismetMathLibrary.VLerp` (`self.K2_GetActorLocation`) (`KismetMathLibrary.MakeVector` _returnvalue_x _returnvalue_y (+ _returnvalue_z 130.0)) _islandspeed)))
    (:`Finished`
      (set `self.HasFinishPlaying` true))))

(event `MoveIsland`
  (goto _label))

(event `self.Sphere.OnComponentBeginOverlap`
  (params (OverlappedComponent :type "PrimitiveComponent Object Reference") (OtherActor :type "Actor Object Reference") (OtherComp :type "PrimitiveComponent Object Reference") (OtherBodyIndex :type Integer) (bFromSweep :type Boolean) (SweepResult :type "HitResult Structure (by ref)"))
  (cast `/Game/Core/Characters/Boat/BP_Boat` OtherActor)
  (if (`self.HasFinishPlaying`)
    (`KismetSystemLibrary.PrintString` "it works")))

(event `self.Sphere.OnComponentEndOverlap`
  (params (OverlappedComponent :type "PrimitiveComponent Object Reference") (OtherActor :type "Actor Object Reference") (OtherComp :type "PrimitiveComponent Object Reference") (OtherBodyIndex :type Integer))
  (cast `/Game/Core/Characters/Boat/BP_Boat` OtherActor)
  (if (`self.HasFinishPlaying`)
    (`KismetSystemLibrary.PrintString` "This one too")))

(fn `UserConstructionScript`)