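; BP_DrowningSpirit is a drowning spirit NPC that the player, piloting BP_Boat, can start a conversation with.
; SpeaktoNPC stores the passed actor, casts the player pawn to BP_Boat and runs StartConversation.
; StartConversation turns the spirit's yaw toward the boat, then has the boat disable input and call up the UI.
; Camera blend, time dilation and FerryMan calls remain as unused, disconnected nodes.
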(event `/Game/Core/Characters/ConversationSection/Libraries/I_Iteractions.Speak to NPC`
  (params (NewHittedActor :type "Actor Object Reference"))
  (set `self.HittedActorRef` NewHittedActor)
  (bind _asbp_boat (cast `/Game/Core/Characters/Boat/BP_Boat` (`GameplayStatics.GetPlayerPawn` 0)))
  (set `self.BoatRef` _asbp_boat)
  (`self.StartConversation`))

(fn `StartConversation`
  (bind (_returnvalue_roll _returnvalue_pitch _returnvalue_yaw) (`KismetMathLibrary.BreakRotator` (`KismetMathLibrary.FindLookAtRotation` (`self.K2_GetActorLocation`) (`self.K2_GetActorLocation` (`self.BoatRef`)))))
  (`self.K2_SetActorRotation` (`KismetMathLibrary.MakeRotator` 0.0 0.0 _returnvalue_yaw))
  (`/Game/Core/Characters/Boat/BP_Boat.DisableInputCallUI` (`self.BoatRef`)))

(fn `UserConstructionScript`)