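; Base passenger NPC character that the player, as the ferryman, can enter and leave a conversation with.
; SpeaktoNPC caches the ferryman and flip-flops between StartConversation and StopConversation.
; Starting turns the NPC toward the player, halts its movement, hides the player mesh, blends the camera to the NPC and ignores move/look input; stopping restores these.
; BeginPlay sets the name text and stores and debug-prints the DT_Passengers last row index.
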(event `self.ReceiveBeginPlay`
  ;[1 1 1] Handles Name
  (bind _outrownames (`DataTableFunctionLibrary.GetDataTableRowNames` "/Game/Core/Characters/ConversationSection/DT_Passengers.DT_Passengers"))
  (bind _returnvalue (`KismetArrayLibrary.Array_LastIndex` _outrownames))
  (`KismetSystemLibrary.PrintString` (`KismetStringLibrary.Conv_IntToString` _returnvalue) true true (struct :`G` 0.66 :`B` 1.0 :`A` 1.0) 60.0)
  (set `self.MaxLength` _returnvalue)
  (`TextRenderComponent.K2_SetText` (`self.NPCName`) (`KismetTextLibrary.Conv_StringToText` (`self.PassengerName`))))

(event `/Game/Core/Characters/ConversationSection/Libraries/I_Iteractions.Speak to NPC`
  ;[1 1 1] Start/stop Conversation
  (bind _asbp_ferry_man_talk (cast `/Game/Core/Characters/ConversationSection/BP_FerryManTalk` (`GameplayStatics.GetPlayerCharacter` 0)))
  (set `self.FerryManRef` _asbp_ferry_man_talk)
  (`/Engine/EditorBlueprintResources/StandardMacros.FlipFlop`
    (:`A`
      (`self.StartConversation`))
    (:`B`
      (`self.StopConversation`))))

(fn `StartConversation`
  (bind _returnvalue (`GameplayStatics.GetPlayerController` 0))
  (bind (_returnvalue_roll _returnvalue_pitch _returnvalue_yaw) (`KismetMathLibrary.BreakRotator` (`KismetMathLibrary.FindLookAtRotation` (`self.K2_GetActorLocation`) (`self.K2_GetActorLocation` (`self.FerryManRef`)))))
  (`self.K2_SetActorRotation` (`KismetMathLibrary.MakeRotator` 0.0 0.0 _returnvalue_yaw))
  ;[1 1 1] Stopping AI movement, hiding mesh of the player, setting the camera to the npc
  (`ActorComponent.SetActive` (`self.CharacterMovement`) false false)
  (`SceneComponent.SetVisibility` (`Character.Mesh` (`self.FerryManRef`)) false false)
  (`PlayerController.SetViewTargetWithBlend` (`GameplayStatics.GetPlayerController` 0) self 0.6 "VTBlend_Linear" 0.0 false)
  ;[1 1 1] Disableling inputs for the player, showing mouse cursor
  (`Controller.SetIgnoreMoveInput` _returnvalue true)
  (`Controller.SetIgnoreLookInput` _returnvalue true))

(fn `StopConversation`
  (bind _returnvalue (`GameplayStatics.GetPlayerController` 0))
  ;[1 1 1] re-enable AI movement, showing mesh of the player, setting the camera back to the player
  (`ActorComponent.SetActive` (`self.CharacterMovement`) true false)
  (`SceneComponent.SetVisibility` (`Character.Mesh` (`self.FerryManRef`)) true false)
  (`PlayerController.SetViewTargetWithBlend` (`GameplayStatics.GetPlayerController` 0) (`self.FerryManRef`) 0.6 "VTBlend_Linear" 0.0 false)
  ;[1 1 1] Enabling inputs for the player, Hidding mouse cursor
  (`Controller.SetIgnoreMoveInput` _returnvalue false)
  (`Controller.SetIgnoreLookInput` _returnvalue false))

(fn `UserConstructionScript`)