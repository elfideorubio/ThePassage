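; BP_Spirit4 is the fourth spirit in the conversation section, whose resolution starts the island's final stage.
; It teleports up once spirit 3 has been spoken to and binds to the player boat's sit and drown dispatchers, filtered by soul ID.
; Sitting sets an animation flag and stops audio; drowning plays a sound and a timeline-driven vertical move.
; Both outcomes mark it spoken to, show "Reach The Island" and call FinalStage.
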(event `self.ReceiveBeginPlay`
  (bind _asbp_boat (cast `/Game/Core/Characters/Boat/BP_Boat` (`GameplayStatics.GetPlayerPawn` 0)))
  (add `/Game/Core/Characters/Boat/BP_Boat.SendNewAnimation` _asbp_boat (delegate `SitOnBoatAnimation`))
  (add `/Game/Core/Characters/Boat/BP_Boat.DrownSoul` _asbp_boat (delegate `DrownSoul`))
  (bind _asbp_fide_game_mode (cast `/Game/Core/Characters/ConversationSection/BP_FideGameMode` (`GameplayStatics.GetGameMode`)))
  (set `self.GameInstanceRef` _asbp_fide_game_mode)
  (set `self.IslandRef` (`self.IslandRef`)))

(event `DrownSoul`
  (params (TimesCalled :type Integer))
  (if (== TimesCalled (`self.IDSoul`))
    (`AudioComponent.SetSound` (`self.Audio`) "/Game/Audio/SFX/OrbSound/Soul_Orb_Move_Sound.Soul_Orb_Move_Sound")
    (`AudioComponent.Play` (`self.Audio`) 0.0)
    (bind (_direction _drownspeed) (`Timeline|Timeline_0`)
      (:`Update`
        (`self.K2_SetActorLocation` (`KismetMathLibrary.VLerp` (`self.K2_GetActorLocation`) (- (`self.K2_GetActorLocation`) (0.0 0.0 -100.0)) _drownspeed)))
      (:`Finished`
        (set `self.HasSpokenWith4` true)
        (message `/Game/Core/Characters/ConversationSection/Libraries/I_Iteractions.ReachTheIslandMessage` (`self.GameInstanceRef`) "Reach The Island")
        (`/Game/Art/Environment/BP_IslandYthen.FinalStage` (`self.IslandRef`))))))

(event `SitOnBoatAnimation`
  (params (TimesCalled :type Integer))
  (if (== TimesCalled (`self.IDSoul`))
    (set `self.Animation4` true)
    (set `self.HasSpokenWith4` true)
    (`AudioComponent.Stop` (`self.Audio`))
    (message `/Game/Core/Characters/ConversationSection/Libraries/I_Iteractions.ReachTheIslandMessage` (`self.GameInstanceRef`) "Reach The Island")
    (`/Game/Art/Environment/BP_IslandYthen.FinalStage` (`self.IslandRef`))))

(event `/Game/Core/Characters/ConversationSection/Libraries/I_Iteractions.HasSpokenTo3`
  (params (HasSpokenTo3 :type Boolean))
  (if HasSpokenTo3
    (`self.TeleportUP` (`self.TeleportLocation`))))

(fn `UserConstructionScript`
  (`parent.UserConstructionScript`))