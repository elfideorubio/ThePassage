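; BP_Spirits2 is the second spirit in a chained conversation section, teleporting up once told that spirit 1 has been spoken to.
; On BeginPlay it binds to the player boat's animation and drown dispatchers, responding only when the call count matches its soul ID.
; It then either switches to its boat-sitting animation or plays a sound and timeline-driven vertical move.
; Both outcomes mark it as spoken to and notify spirit 3.
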(event `self.ReceiveBeginPlay`
  (bind _asbp_boat (cast `/Game/Core/Characters/Boat/BP_Boat` (`GameplayStatics.GetPlayerPawn` 0)))
  (add `/Game/Core/Characters/Boat/BP_Boat.SendNewAnimation` _asbp_boat (delegate `SitOnBoatAnimation`))
  (add `/Game/Core/Characters/Boat/BP_Boat.DrownSoul` _asbp_boat (delegate `DrownSoul`))
  (set `self.Spirit3Ref` (`self.Spirit3Ref`)))

(event `DrownSoul`
  (params (TimesCalled :type Integer))
  (if (== TimesCalled (`self.IDSoul`))
    (`AudioComponent.SetSound` (`self.Audio`) "/Game/Audio/SFX/OrbSound/Soul_Orb_Move_Sound.Soul_Orb_Move_Sound")
    (`AudioComponent.Play` (`self.Audio`) 0.0)
    (bind (_direction _drownspeed) (`Timeline|Timeline_0`)
      (:`Update`
        (`self.K2_SetActorLocation` (`KismetMathLibrary.VLerp` (`self.K2_GetActorLocation`) (- (`self.K2_GetActorLocation`) (0.0 0.0 -500.0)) _drownspeed))
        (set `self.HasSpokenWith2` true)
        (`/Game/Core/Characters/ConversationSection/Libraries/I_Iteractions.HasSpokenTo2` (`self.Spirit3Ref`) true)))))

(event `SitOnBoatAnimation`
  (params (TimesCalled :type Integer))
  (if (== TimesCalled (`self.IDSoul`))
    (set `self.Animation2` true)
    (set `self.HasSpokenWith2` true)
    (`AudioComponent.Stop` (`self.Audio`))
    (`/Game/Core/Characters/ConversationSection/Libraries/I_Iteractions.HasSpokenTo2` (`self.Spirit3Ref`) true)))

(event `/Game/Core/Characters/ConversationSection/Libraries/I_Iteractions.HasSpokenTo1`
  (params (HasSpoken1 :type Boolean))
  (if HasSpoken1
    (`self.TeleportUP` 4420.0)))

(fn `UserConstructionScript`
  (`parent.UserConstructionScript`))