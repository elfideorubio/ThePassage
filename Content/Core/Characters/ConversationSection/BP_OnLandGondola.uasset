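; BP_OnLandGondola is the gondola actor in the conversation section that takes aboard passengers sent by the ferryman.
; On BeginPlay it binds to the SendHimToTheBoat dispatcher of the player's BP_FerryManTalk character.
; Each received actor is attached to the gondola with relative transforms kept.
; For BP_PassengersBaseClass actors, it also appends the passenger name to a list and copies that list into BP_GameInstance's Passengers.
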(event `self.ReceiveBeginPlay`
  (bind _asbp_ferry_man_talk (cast `/Game/Core/Characters/ConversationSection/BP_FerryManTalk` (`GameplayStatics.GetPlayerCharacter` 0)))
  (set `self.FerryManRef` _asbp_ferry_man_talk)
  (add `/Game/Core/Characters/ConversationSection/BP_FerryManTalk.SendHimToTheBoat` (`self.FerryManRef`) (delegate `SendHimToTheBoat_Event_0`)))

(event `SendHimToTheBoat_Event_0`
  (params (HittedActor :type "Actor Object Reference"))
  (bind _output_get (set `self.HittedActorRef` HittedActor))
  (`self.K2_AttachToActor` _output_get self "None" "KeepRelative" "KeepRelative" "KeepRelative" true)
  (bind _asbp_passengers_base_class (cast `/Game/Core/Characters/ConversationSection/BP_PassengersBaseClass` (`self.HittedActorRef`)))
  (`KismetArrayLibrary.Array_Add` (`self.NameOfActors`) (`/Game/Core/Characters/ConversationSection/BP_PassengersBaseClass.PassengerName` _asbp_passengers_base_class))
  (bind _asbp_game_instance (cast `/Game/Core/Characters/ConversationSection/BP_GameInstance` (`GameplayStatics.GetGameInstance`)))
  (set `/Game/Core/Characters/ConversationSection/BP_GameInstance.Passengers` (`self.NameOfActors`) _asbp_game_instance))

(fn `UserConstructionScript`)