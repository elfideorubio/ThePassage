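; Spawner actor that populates the area around it with passenger NPCs when play begins.
; It loops once per row in DT_Passengers, each time picking a random row by a numeric row name, so passengers can repeat.
; Each found row spawns a BP_PassengersBaseClass at a random reachable navmesh point near the spawner, passing in the row's NPC name.
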(event `self.ReceiveBeginPlay`
  (bind _outrownames (`DataTableFunctionLibrary.GetDataTableRowNames` "/Game/Core/Characters/ConversationSection/DT_Passengers.DT_Passengers"))
  (set `self.MaxNumberOfPassengers` (`KismetArrayLibrary.Array_LastIndex` _outrownames))
  (for _ (range (+ (`self.MaxNumberOfPassengers`) 1))
    (bind _returnvalue (`|GetDataTableRow` "/Game/Core/Characters/ConversationSection/DT_Passengers.DT_Passengers" (`KismetStringLibrary.Conv_StringToName` (`KismetStringLibrary.Conv_IntToString` (`KismetMathLibrary.RandomIntegerInRange` 0 (`self.MaxNumberOfPassengers`)))))
      (:`then`
        (`|SpawnActorFromClass` "/Game/Core/Characters/ConversationSection/BP_PassengersBaseClass.BP_PassengersBaseClass_C" (`KismetMathLibrary.MakeTransform` (`NavigationSystemV1.K2_GetRandomReachablePointInRadius` (`SceneComponent.K2_GetComponentLocation` (`self.DefaultSceneRoot`)) 300.0 null null)) "Undefined" "OverrideRootScale" null (`.NPCName_5_281319064B7FC790F6AAD9B663843147` (break `/Game/Core/Characters/ConversationSection/Struc_Passengers` _returnvalue)) null)))))

(fn `UserConstructionScript`)