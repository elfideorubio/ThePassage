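; Base class for spirit NPCs that hold a conversation with the player's boat.
; SpeaktoNPC caches the interacted actor and the BP_Boat pawn, runs StartConversation, then switches off capsule gravity and collision.
; StartConversation yaws the spirit toward the boat, blends the view target to itself, disables boat input and passes its name, question and response to the UI call.
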(event `self.ReceiveBeginPlay`)

(event `/Game/Core/Characters/ConversationSection/Libraries/I_Iteractions.Speak to NPC`
  (params (NewHittedActor :type "Actor Object Reference"))
  (set `self.HittedActorRef` NewHittedActor)
  (bind _asbp_boat (cast `/Game/Core/Characters/Boat/BP_Boat` (`GameplayStatics.GetPlayerPawn` 0)))
  (set `self.BoatRef` _asbp_boat)
  (`self.StartConversation`)
  (`PrimitiveComponent.SetEnableGravity` (`self.CapsuleComponent`) false)
  (`PrimitiveComponent.SetCollisionEnabled` (`self.CapsuleComponent`) "NoCollision"))

(fn `StartConversation`
  (bind (_returnvalue_roll _returnvalue_pitch _returnvalue_yaw) (`KismetMathLibrary.BreakRotator` (`KismetMathLibrary.FindLookAtRotation` (`self.K2_GetActorLocation`) (`self.K2_GetActorLocation` (`self.BoatRef`)))))
  (`self.K2_SetActorRotation` (`KismetMathLibrary.MakeRotator` 0.0 0.0 _returnvalue_yaw))
  (`PlayerController.SetViewTargetWithBlend` (`GameplayStatics.GetPlayerController` 0) self 0.6 "VTBlend_Linear" 0.0 false)
  (`/Game/Core/Characters/Boat/BP_Boat.DisableInputCallUI` (`self.BoatRef`))
  (`self.Callui` (`self.Question`) (`self.DisplayName`) (`self.Reponse`)))

(fn `UserConstructionScript`)