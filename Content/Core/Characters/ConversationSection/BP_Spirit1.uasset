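; BP_Spirit1 is a soul in the conversation section that reacts to the boat pawn's decision to seat or drown it.
; On BeginPlay it binds to BP_Boat's animation and drown events, then calls TeleportUP after a delay.
; When the ID matches, it either enables its sitting animation and stops audio, or plays a sound while a timeline shifts it vertically.
; Both outcomes mark it as spoken with and notify Spirit2.
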(event `self.ReceiveBeginPlay`
  (`|ExecutionSequence`
    (:`then_0`
      ;[1 1 1] Comment
      (bind _asbp_boat (cast `/Game/Core/Characters/Boat/BP_Boat` (`GameplayStatics.GetPlayerPawn` 0)))
      (add `/Game/Core/Characters/Boat/BP_Boat.SendNewAnimation` _asbp_boat (delegate `SitOnBoatAnimation`))
      (add `/Game/Core/Characters/Boat/BP_Boat.DrownSoul` _asbp_boat (delegate `DrownSoul`))
      (set `self.Spirit2` (`self.Spirit2`)))
    (:`then_1`
      (`KismetSystemLibrary.Delay` 3.0)
      (`self.TeleportUP` (`self.TeleportLocation`)))))

(event `DrownSoul`
  (params (TimesCalled :type Integer))
  ;[1 1 1] Comment
  (if (== TimesCalled (`self.IDSoul`))
    (`AudioComponent.SetSound` (`self.Audio`) "/Game/Audio/SFX/OrbSound/Soul_Orb_Move_Sound.Soul_Orb_Move_Sound")
    (`AudioComponent.Play` (`self.Audio`) 0.0)
    (bind (_direction _drownspeed) (`Timeline|Drown`)
      (:`Update`
        (`self.K2_SetActorLocation` (`KismetMathLibrary.VLerp` (`self.K2_GetActorLocation`) (- (`self.K2_GetActorLocation`) (0.0 0.0 -500.0)) _drownspeed))
        (bind _output_get (set `self.HasSpokenWith1` true))
        (`self.HasInteractedWith1` _output_get)
        (`/Game/Core/Characters/ConversationSection/Libraries/I_Iteractions.HasSpokenTo1` (`self.Spirit2`) true)))))

(event `SitOnBoatAnimation`
  (params (TimesCalled :type Integer))
  ;[1 1 1] Comment
  (if (== TimesCalled (`self.IDSoul`))
    (set `self.Animation1` true)
    (set `self.HasSpokenWith1` true)
    (`/Game/Core/Characters/ConversationSection/Libraries/I_Iteractions.HasSpokenTo1` (`self.Spirit2`) true)
    (`AudioComponent.Stop` (`self.Audio`))))

(fn `UserConstructionScript`
  (`parent.UserConstructionScript`))