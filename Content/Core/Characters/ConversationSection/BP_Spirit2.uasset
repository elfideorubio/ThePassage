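; BP_Spirit2 is a spirit character in the conversation section that reacts to the player's boat.
; On BeginPlay it casts the player pawn to BP_Boat and binds to its SendNewAnimation dispatcher.
; When the dispatcher fires, it sets the Animation2 flag to true, ignoring the passenger count it receives.
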(event `self.ReceiveBeginPlay`
  (bind _asbp_boat (cast `/Game/Core/Characters/Boat/BP_Boat` (`GameplayStatics.GetPlayerPawn` 0)))
  (add `/Game/Core/Characters/Boat/BP_Boat.SendNewAnimation` _asbp_boat (delegate `AnimationToTrue`)))

(event `AnimationToTrue`
  (params (NumbPassengers :type Integer))
  (set `self.Animation2` true))

(fn `UserConstructionScript`
  (`parent.UserConstructionScript`))