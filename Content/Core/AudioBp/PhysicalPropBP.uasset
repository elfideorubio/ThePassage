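; PhysicalPropBP is a component that plays impact sounds when its owning physics prop hits something hard enough.
; Tick stores the sum of the static mesh's signed velocity axes as a speed estimate and prints it every frame.
; On a hit, high values play FastImpact, while lower ones randomly play Settle or Strike with volume scaled by that estimate.
; Sounds play at the actor's location; the hit surface type is stored but unused here.
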(event `self.ReceiveBeginPlay`
  ;[1 1 1] ImpactAudio
  (add `Actor.OnActorHit` (`self.GetOwner`) (delegate `OBJECTCOLLIDES`)))

(event `OBJECTCOLLIDES`
  (params (SelfActor :type "Actor Object Reference") (OtherActor :type "Actor Object Reference") (NormalImpulse :type "Vector Structure") (Hit :type "HitResult Structure (by ref)"))
  (bind _ve (`self.ve`))
  (bind _impactedvolume (`self.ImpactedVolume`))
  (bind _ve_2 (`self.ve`))
  ;[1 1 1] ImpactAudio
  (set `self.PhysSurfaceHit` (`GameplayStatics.GetSurfaceType` Hit))
  (if (> (`KismetMathLibrary.VSize` NormalImpulse) 1000.0)
    (set `self.HitLocation` (`Actor.K2_GetActorLocation` SelfActor))
    (if (or (>= _ve 1600.0) (<= _ve -1600.0))
      (`GameplayStatics.PlaySoundAtLocation` "/Game/FirstPersonBP/SoundBooth/Sounds/WoodBlock/FastImpact.FastImpact" (`self.HitLocation`) (struct) 1.0 1.0 0.0 null null null)
      (else
        (if (< (`self.ve`) 0.0)
          (set `self.ImpactedVolume` (/ (* _ve_2 -1.0) 800.0))
          (else
            (set `self.ImpactedVolume` (/ _ve_2 800.0))))
        (if (`KismetMathLibrary.RandomBool`)
          (`GameplayStatics.PlaySoundAtLocation` "/Game/FirstPersonBP/SoundBooth/Sounds/WoodBlock/Settle.Settle" (`self.HitLocation`) (struct) _impactedvolume 1.0 0.0 null null null)
          (else
            (`GameplayStatics.PlaySoundAtLocation` "/Game/FirstPersonBP/SoundBooth/Sounds/WoodBlock/Strike.Strike" (`self.HitLocation`) (struct) _impactedvolume 1.0 0.0 null null null)))))))

(event `self.ReceiveTick`
  (params (DeltaSeconds :type "Float (single-precision)"))
  ;[1 1 1] StateChecks
  (bind _returnvalue (`PrimitiveComponent.GetPhysicsLinearVelocity` (`Actor.GetComponentByClass` (`self.GetOwner`) "/Script/Engine.StaticMeshComponent") "None"))
  (bind _output_get (set `self.ve` (+ (.x _returnvalue) (.y _returnvalue) (.z _returnvalue))))
  (`KismetSystemLibrary.PrintString` (`KismetStringLibrary.Conv_DoubleToString` _output_get)))